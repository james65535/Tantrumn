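; AI controller for Tantrumn bots that picks a behavior tree and blackboard by game mode: Battle, Race or Dodgeball.
; Race mode also seeds Destination with the level end trigger's location, while the Battle destination helper's write is disconnected.
; AI perception stores a sensed floating platform as TargetPlatform when the blackboard is looking for one and none is set.
; Forgotten-perception events only log and leave TargetPlatform uncleared.
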(event `self.ReceiveBeginPlay`
  (bind _returnvalue (`GameplayStatics.GetGameMode`))
  ;[1 1 1] Battle AI
  (cast `/Game/Tantrumn/Blueprints/GameModes/BP_TantrumnBattleGameMode` _returnvalue
    (:`then`
      (`self.RunBehaviorTree` "/Game/Tantrumn/Blueprints/AI/BTrees/BT_TantrumnBattle.BT_TantrumnBattle")
      (`self.UseBlackboard` "/Game/Tantrumn/Blueprints/AI/Blackboards/BB_TantrumnBattle.BB_TantrumnBattle")
      (`self.SetThrowableObjectAsDestination`))
    (:`CastFailed`
      ;[1 1 1] Race AI
      (cast `/Game/Tantrumn/Blueprints/GameModes/BP_TantrumnRaceGameMode` _returnvalue
        (:`then`
          (`self.RunBehaviorTree` "/Game/Tantrumn/Blueprints/AI/BTrees/BT_TantrumnRacePlatform.BT_TantrumnRacePlatform")
          (`self.UseBlackboard` "/Game/Tantrumn/Blueprints/AI/Blackboards/BB_TantrumnRace.BB_TantrumnRace")
          ;;[1 0.5573 0.5573] Review
          (`self.SetRaceEndAsDestination`))
        (:`CastFailed`
          ;[1 1 1] Dodgeball AI
          (cast `/Game/Tantrumn/Blueprints/GameModes/BP_TantrumnDodgeBallGameMode` _returnvalue
            (:`then`
              (`self.RunBehaviorTree` "/Game/Tantrumn/Blueprints/AI/BTrees/BT_TantrumnDodgeball.BT_TantrumnDodgeball")
              (`self.UseBlackboard` "/Game/Tantrumn/Blueprints/AI/Blackboards/BB_TantrumnDodgeBall.BB_TantrumnDodgeBall"))
            (:`CastFailed`
              (`KismetSystemLibrary.PrintString` "AI Controller Failed to Determine Game Mode"))))))))

(event `self.AIPerceptionComponent.OnTargetPerceptionUpdated`
  (params (Actor :type "Actor Object Reference") (Stimulus :type "AIStimulus Structure"))
  (bind _returnvalue (`AIBlueprintHelperLibrary.GetBlackboard` null))
  ;[1 1 1] Add AI sense sight moving platform to BlackBoard if BB value is not already set
  (if (`BlackboardComponent.GetValueAsBool` _returnvalue "IsLookingForPlatform")
    (`/Engine/EditorBlueprintResources/StandardMacros.IsValid` (`BlackboardComponent.GetValueAsObject` _returnvalue "TargetPlatform")
      (:`Is Not Valid`
        (if true
          (bind _asfloating_platform (cast `FloatingPlatform` Actor))
          (`BlackboardComponent.SetValueAsObject` (`AIBlueprintHelperLibrary.GetBlackboard` null) "TargetPlatform" _asfloating_platform))))))

(event `self.AIPerceptionComponent.OnTargetPerceptionForgotten`
  (params (Actor :type "Actor Object Reference"))
  (bind _returnvalue (`BlackboardComponent.GetValueAsObject` (`AIBlueprintHelperLibrary.GetBlackboard` null) "TargetPlatform"))
  (bind _returnvalue_2 (`KismetSystemLibrary.GetObjectName` _returnvalue))
  ;[1 1 1] Clear out stale moving platform Blackboard Value
  (`/Engine/EditorBlueprintResources/StandardMacros.IsValid` _returnvalue
    (:`Is Valid`
      (if (`KismetStringLibrary.EqualEqual_StrStr` (`KismetSystemLibrary.GetObjectName` Actor) _returnvalue_2)
        (`KismetSystemLibrary.LogString` (`KismetStringLibrary.Concat_StrStr` "AISight forgot Platform: " _returnvalue_2))))
    (:`Is Not Valid`
      (`KismetSystemLibrary.LogString` "AISight forgot something but had no target platform"))))

(fn `SetRaceEndAsDestination`
  (bind _outactors (`GameplayStatics.GetAllActorsOfClass` "/Script/Tantrumn.TantrumnLevelEndTrigger"))
  ;[1 1 1] Now handled by EQS
  (if (> (`KismetArrayLibrary.Array_Length` _outactors) 0)
    (`BlackboardComponent.SetValueAsVector` (`self.Blackboard`) "Destination" (`self.K2_GetActorLocation` (`|GetArrayItem` _outactors)))))

(fn `SetThrowableObjectAsDestination`
  (bind _outactors (`GameplayStatics.GetAllActorsOfClass` "/Game/Tantrumn/Blueprints/InteracableObjects/BP_ThrowableActor.BP_ThrowableActor_C")))

(fn `UserConstructionScript`)