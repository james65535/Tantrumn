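; AI controller for Tantrumn D-Ball worker bots that picks its behavior from the current game mode.
; On BeginPlay it runs the Battle or Race behavior tree and blackboard, and in races seeds Destination with the level end trigger's location.
; Each Tick it mirrors the game state's in-play status into the IsPlaying blackboard key.
; The throwable-targeting helper is unused, noted as now handled by EQS.
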(event `self.ReceiveBeginPlay`
  (bind _returnvalue (`GameplayStatics.GetGameMode`))
  (cast `/Game/Tantrumn/Blueprints/GameModes/BP_TantrumnBattleGameMode` _returnvalue
    (:`then`
      ;[1 1 1] Battle AI
      (`self.RunBehaviorTree` "/Game/Tantrumn/Blueprints/AI/BTrees/BT_TantrumnBattle.BT_TantrumnBattle")
      (`self.UseBlackboard` "/Game/Tantrumn/Blueprints/AI/Blackboards/BB_TantrumnBattle.BB_TantrumnBattle"))
    (:`CastFailed`
      ;[1 1 1] Race AI
      (cast `/Game/Tantrumn/Blueprints/GameModes/BP_TantrumnRaceGameMode` _returnvalue
        (:`then`
          (`self.RunBehaviorTree` "/Game/Tantrumn/Blueprints/AI/BTrees/BT_TantrumnRace.BT_TantrumnRace")
          (`self.UseBlackboard` "/Game/Tantrumn/Blueprints/AI/Blackboards/BB_TantrumnRace.BB_TantrumnRace")
          (`self.SetRaceEndAsDestination`))
        (:`CastFailed`
          (`KismetSystemLibrary.PrintString` "AI Controller Failed to Determine Game Mode"))))))

(event `self.ReceiveTick`
  (params (DeltaSeconds :type "Float (single-precision)"))
  (bind _asbp_tantrumn_game_state_base (cast `/Game/Tantrumn/Blueprints/GameState/BP_TantrumnGameStateBase` (`GameplayStatics.GetGameState`)))
  (bind _blackboard (`self.Blackboard`)
    (:`then`
      (`BlackboardComponent.SetValueAsBool` _blackboard "IsPlaying" (`TantrumnGameStateBase.IsGameInPlay` _asbp_tantrumn_game_state_base)))
    (:`else`)))

(fn `SetRaceEndAsDestination`
  (bind _outactors (`GameplayStatics.GetAllActorsOfClass` "/Script/Tantrumn.TantrumnLevelEndTrigger"))
  ;[1 1 1] Now handled by EQS
  (if (> (`KismetArrayLibrary.Array_Length` _outactors) 0)
    (`BlackboardComponent.SetValueAsVector` (`self.Blackboard`) "Destination" (`self.K2_GetActorLocation` (`|GetArrayItem` _outactors)))))

(fn `SetThrowableObjectAsDestination`
  (bind _outactors (`GameplayStatics.GetAllActorsOfClass` "/Game/Tantrumn/Blueprints/InteracableObjects/BP_ThrowableActor.BP_ThrowableActor_C")))

(fn `UserConstructionScript`)