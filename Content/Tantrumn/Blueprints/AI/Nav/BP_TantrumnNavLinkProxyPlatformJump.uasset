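; Smart nav link proxy that flags platform jumps for Tantrumn AI agents.
; When an agent reaches the link, it writes the destination to its BP_TantrumnAIController's Blackboard and sets flags marking it jump-reachable and the AI as looking for a platform.
; Path following then resumes immediately, also for agents without that controller or a valid Blackboard, so the jump itself is handled outside this Blueprint.
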(event `self.ReceiveSmartLinkReached`
  (params (Agent :type "Actor Object Reference") (Destination :type "Vector Structure (by ref)"))
  (bind _asbp_tantrumn_aicontroller (cast `/Game/Tantrumn/Blueprints/Controllers/BP_TantrumnAIController` (`AIBlueprintHelperLibrary.GetAIController` Agent))
    (:`then`
      (bind _blackboard (`AIController.Blackboard` _asbp_tantrumn_aicontroller)
        (:`then`
          (`BlackboardComponent.SetValueAsVector` _blackboard "FinalNavlinkDestination" Destination)
          (`BlackboardComponent.SetValueAsBool` _blackboard "IsDestinationReachableByJump" true)
          (`BlackboardComponent.SetValueAsBool` _blackboard "IsLookingForPlatform" true)
          (`self.ResumePathFollowing` _asbp_tantrumn_aicontroller))
        (:`else`
          (`self.ResumePathFollowing` Agent :!label _label))))
    (:`CastFailed`
      (goto _label))))

(fn `UserConstructionScript`)