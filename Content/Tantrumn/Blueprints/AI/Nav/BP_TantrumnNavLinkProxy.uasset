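; Nav link proxy that tells Tantrumn AI agents to avoid an obstacle when they reach a smart link.
; On SmartLinkReached it gets the agent's BP_TantrumnAIController and writes its blackboard: it sets the ShouldAvoidObstacle flag and stores the link destination as ObstacleAvoidanceDestination.
; The proxy performs no movement itself; a leftover, disconnected branch that made BP_Player jump never runs.
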(event `self.ReceiveSmartLinkReached`
  (params (Agent :type "Actor Object Reference") (Destination :type "Vector Structure (by ref)"))
  (bind _asbp_tantrumn_aicontroller (cast `/Game/Tantrumn/Blueprints/Controllers/BP_TantrumnAIController` (`AIBlueprintHelperLibrary.GetAIController` Agent)))
  (bind _returnvalue (`AIBlueprintHelperLibrary.GetBlackboard` _asbp_tantrumn_aicontroller))
  (`BlackboardComponent.SetValueAsBool` _returnvalue "ShouldAvoidObstacle" true)
  (`BlackboardComponent.SetValueAsVector` _returnvalue "ObstacleAvoidanceDestination" Destination))

(fn `UserConstructionScript`)