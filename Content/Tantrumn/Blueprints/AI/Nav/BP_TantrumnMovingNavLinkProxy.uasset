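; Nav link proxy that launches Tantrumn characters across a smart link whose endpoint is meant to follow a moving actor.
; A Timeline started on BeginPlay uses its updates to copy ActorToTrack's world Y offset into the first point link's Left point and RightSphere's relative location.
; When an agent reaches the link, it is launched after a short delay on a suggested projectile arc to the destination.
; Both paths print debug strings.
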(event `self.ReceiveSmartLinkReached`
  (params (Agent :type "Actor Object Reference") (Destination :type "Vector Structure (by ref)"))
  (`KismetSystemLibrary.PrintString` "Smart Link Reached")
  (bind _astantrumn_character_base (cast `TantrumnCharacterBase` Agent))
  (bind _outlaunchvelocity (`GameplayStatics.SuggestProjectileVelocity_CustomArc` (`self.K2_GetActorLocation` _astantrumn_character_base) Destination))
  (`KismetSystemLibrary.Delay` 0.1)
  (`Character.LaunchCharacter` _astantrumn_character_base _outlaunchvelocity false false))

(event `self.ReceiveBeginPlay`
  (bind (_returnvalue_x _returnvalue_y) (`KismetMathLibrary.BreakVector` (`self.K2_GetActorLocation`)))
  (bind _output_left (break `NavigationLink` (`|GetArrayItem` (`self.PointLinks`))))
  (`Timeline|Timeline` :`NewTime` 10000.0 :!via `PlayFromStart`
    (:`Update`
      (bind _actortotrack (`self.ActorToTrack`)
        (:`then`
          (bind (_returnvalue_x_2 _returnvalue_y_2) (`KismetMathLibrary.BreakVector` (- (`self.K2_GetActorLocation` _actortotrack) (`KismetMathLibrary.MakeVector` _returnvalue_x _returnvalue_y))))
          (bind _output_get (set `self.MovingPointLocation` (`KismetMathLibrary.MakeVector` 0.0 _returnvalue_y_2)))
          (`KismetMathLibrary.Vector_Set` _output_left (.x _output_get) (.y _output_get) (.z _output_get))
          (`SceneComponent.K2_SetRelativeLocation` (`self.RightSphere`) (`self.MovingPointLocation`) false false)
          (`KismetSystemLibrary.PrintString` (`KismetStringLibrary.Conv_VectorToString` _output_left)))
        (:`else`)))))

(fn `UserConstructionScript`)