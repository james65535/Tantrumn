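; Nav link proxy in Tantrumn that makes a BP_Player agent jump when it reaches the smart link.
; SmartLinkReached casts the agent to BP_Player and calls Jump, with debug prints on entry and on a failed cast.
; An unconnected chain, which never runs, would instead launch the character toward the link destination using a suggested arc velocity scaled by JumpBoost, after a short delay.
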(event `self.ReceiveSmartLinkReached`
  (params (Agent :type "Actor Object Reference") (Destination :type "Vector Structure (by ref)"))
  (`KismetSystemLibrary.PrintString` "Hello")
  (bind _asbp_player (cast `/Game/Tantrumn/Blueprints/Characters/BP_Player` Agent)
    (:`then`
      (`Character.Jump` _asbp_player))
    (:`CastFailed`
      (`KismetSystemLibrary.PrintString` "Navlink Cast to BP Player Failed"))))

(fn `UserConstructionScript`)