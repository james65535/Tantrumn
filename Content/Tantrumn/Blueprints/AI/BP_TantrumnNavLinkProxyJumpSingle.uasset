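; Smart nav link proxy that makes Tantrumn AI characters jump when they reach the link while path following.
; On smart link reached, it casts the agent to TantrumnCharacterBase, calls Jump and immediately resumes path following.
; Disconnected leftover nodes would launch the character on a suggested projectile arc toward a tracked actor or disable the smart link, but they never run.
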(event `self.ReceiveSmartLinkReached`
  (params (Agent :type "Actor Object Reference") (Destination :type "Vector Structure (by ref)"))
  (`KismetSystemLibrary.PrintString` "Smart Link Reached")
  (bind _astantrumn_character_base (cast `TantrumnCharacterBase` Agent))
  (`Character.Jump` _astantrumn_character_base)
  (`self.ResumePathFollowing` _astantrumn_character_base))

(event `self.ReceiveBeginPlay`)

(fn `UserConstructionScript`)