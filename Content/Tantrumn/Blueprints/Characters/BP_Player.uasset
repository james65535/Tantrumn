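; BP_Player is the Tantrumn player character Blueprint, adding aim handling and jump diagnostics.
; Jump, land and Tick logic print takeoff velocity, apex time, air time and distance as on-screen debug text.
; Tick detects aim-state changes, moving the follow camera between two anchor components and toggling controller-facing versus movement-facing rotation.
; An unused Hold macro separates taps from holds with gates and a retriggerable delay, and a stun-check test is left unconnected.
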(event `self.ReceiveBeginPlay`
  ;[1 1 1] Prototype test for custom character movement component
)

(event `self.OnJumped`
  ;[1 1 1] Calculations used to display Jump Length
  (set `self.JumpStartTime` (`GameplayStatics.GetTimeSeconds`))
  (set `self.StartPosition` (`self.K2_GetActorLocation`))
  (`KismetSystemLibrary.PrintString` (`KismetStringLibrary.Concat_StrStr` "Velocity: " (`KismetStringLibrary.Conv_VectorToString` (`self.GetVelocity`))) true true (struct :`R` 0.113725 :`G` 0.086275 :`B` 0.807843 :`A` 1.0) 10.0))

(event `self.OnLanded`
  (params (Hit :type "HitResult Structure (by ref)"))
  ;[1 1 1] Display Jump Time
  (`KismetSystemLibrary.PrintString` (`KismetStringLibrary.Concat_StrStr` "JumpTime: " (`KismetStringLibrary.Conv_DoubleToString` (- (`GameplayStatics.GetTimeSeconds`) (`self.JumpStartTime`)))) true true (struct :`R` 1.0 :`G` 0.117647 :`B` 0.219608 :`A` 1.0) 10.0)
  ;[1 1 1] Display Jump Length
  (`KismetSystemLibrary.PrintString` (`KismetStringLibrary.Concat_StrStr` "JumpDistance: " (`KismetStringLibrary.Conv_DoubleToString` (`KismetMathLibrary.VSize` (- (`self.K2_GetActorLocation`) (`self.StartPosition`))))) true true (struct :`G` 0.66 :`B` 1.0 :`A` 1.0) 10.0))

(event `self.ReceiveTick`
  (params (DeltaSeconds :type "Float (single-precision)"))
  (bind (_returnvalue_x _returnvalue_y _returnvalue_z) (`KismetMathLibrary.BreakVector` (`self.GetVelocity`)))
  (bind _returnvalue (`self.IsAiming`))
  (bind (_lastvelocity_x _lastvelocity_y _lastvelocity_z) (`KismetMathLibrary.BreakVector` (`self.Lastvelocity`)))
  ;[1 1 1] Display Jump Apex Time
  (if (and (> _lastvelocity_z 0.0) (< _returnvalue_z 0.0))
    (`KismetSystemLibrary.PrintString` (`KismetStringLibrary.Concat_StrStr` "ApexTime: " (`KismetStringLibrary.Conv_DoubleToString` (- (`GameplayStatics.GetTimeSeconds`) (`self.JumpStartTime`)))) true true (struct :`R` 0.043137 :`G` 0.552941 :`B` 0.05098 :`A` 1.0) 10.0))
  (set `self.Lastvelocity` (`self.GetVelocity`))
  (if (!= _returnvalue (`self.bIsAiming`))
    (if _returnvalue
      (`self.OnStartAim`)
      (else
        (`self.OnStopAim`)))
    (set `self.bIsAiming` _returnvalue)))

(fn `OnStartAim`
  (bind _tantrumncharmovecomp (`self.TantrumnCharMoveComp`))
  (`SceneComponent.K2_SetRelativeLocation` (`self.FollowCamera`) (`SceneComponent.RelativeLocation` (`self.AimCamLocation`)) false false)
  (set `CharacterMovementComponent.bUseControllerDesiredRotation` true _tantrumncharmovecomp)
  (set `CharacterMovementComponent.bOrientRotationToMovement` false _tantrumncharmovecomp))

(fn `OnStopAim`
  (bind _tantrumncharmovecomp (`self.TantrumnCharMoveComp`))
  (`SceneComponent.K2_SetRelativeLocation` (`self.FollowCamera`) (`SceneComponent.RelativeLocation` (`self.FollowCamLocation`)) false false)
  (set `CharacterMovementComponent.bUseControllerDesiredRotation` false _tantrumncharmovecomp)
  (set `CharacterMovementComponent.bOrientRotationToMovement` true _tantrumncharmovecomp))

(fn `UserConstructionScript`)