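; Moving platform actor with configurable mesh, material, control points and duration, paired with optional nav link references to and from the platform.
; The construction script feeds these settings into the mesh and InterpToMovement component.
; From BeginPlay, a Timeline's updates copy each link's Left and Right points to the relative locations of cube (to-platform) and sphere (from-platform) components.
; The graph only reads the links, never modifying them.
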(event `self.ReceiveBeginPlay`
  (`Timeline|Timeline` :`NewTime` 60.0
    (:`Update`
      (`|ExecutionSequence`
        (:`then_0`
          (bind _navlinktoplatform (`self.NavLinkToPlatform`)
            (:`then`
              (for _array_element (`NavLinkComponent.Links` _navlinktoplatform)
                (bind (_left _right) (break `NavigationLink` _array_element))
                (`SceneComponent.K2_SetRelativeLocation` (`self.CubeLeftToPlatform`) _left false false)
                (`SceneComponent.K2_SetRelativeLocation` (`self.CubeRightToPlatform`) _right false false)))
            (:`else`)))
        (:`then_1`
          (bind _navlinkfromplatform (`self.NavLinkFromPlatform`)
            (:`then`
              (for _array_element_2 (`NavLinkComponent.Links` _navlinkfromplatform)
                (bind (_left_2 _right_2) (break `NavigationLink` _array_element_2))
                (`SceneComponent.K2_SetRelativeLocation` (`self.SphereLeftFromtPlatform`) _left_2 false false)
                (`SceneComponent.K2_SetRelativeLocation` (`self.SphereRightFromPlatform`) _right_2 false false)))
            (:`else`)))))))

(fn `UserConstructionScript`
  (bind _interptomovement (`self.InterpToMovement`))
  (bind _moving_platform (`self.Moving_Platform`))
  (set `InterpToMovementComponent.ControlPoints` (`self.Control Points`) _interptomovement)
  (set `InterpToMovementComponent.Duration` (`self.Duration`) _interptomovement)
  (`PrimitiveComponent.SetMaterial` _moving_platform 0 (`self.Material`))
  (`StaticMeshComponent.SetStaticMesh` _moving_platform (`self.Static Mesh`)))